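; BP_Target is a shooting target that falls when damaged and raises itself again.
; Any damage while upright sets IsDown and plays a timeline that rotates ArmPivot 90 degrees.
; When the fall finishes, it waits three seconds, clears IsDown and reverses the timeline to stand back up.
; Further damage is ignored while the target is down.
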(event `self.ReceiveAnyDamage`
  (params (Damage :type "Float (single-precision)") (DamageType :type "DamageType Object Reference") (InstigatedBy :type "Controller Object Reference") (DamageCauser :type "Actor Object Reference"))
  (if (not (`self.bIsDown`))
    (set `self.bIsDown` true)
    (bind (_direction _newtrack_0) (`Timeline|TL_Fall` :!label _label)
      (:`Update`
        (`SceneComponent.K2_SetRelativeRotation` (`self.ArmPivot`) (`KismetMathLibrary.RLerp` (struct) (struct :`Pitch` -90.0) _newtrack_0) false false))
      (:`Finished`
        (if (`self.bIsDown`)
          (`KismetSystemLibrary.Delay` 3.0)
          (set `self.bIsDown` false)
          (goto _label :!via `Reverse`))))))

(fn `UserConstructionScript`)