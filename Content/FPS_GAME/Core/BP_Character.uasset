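; First-person player character for an FPS, driven by Enhanced Input, that creates the HUD and attaches inventory weapons to its arms.
; Held fire loops montage, camera hitscan, damage, impulse and destruction field, gated by ammo, reload, holster, running and wall proximity.
; Sprint and crouch adjust speed, with timelines for FOV and capsule height; fast crouches trigger slides.
; Tick pitches the camera pivot, detects walls and applies gamepad aim assist toward Enemy-tagged actors.
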(event `self.ReceiveBeginPlay`
  (`EnhancedInputSubsystemInterface.AddMappingContext` (pcsubsystem `EnhancedInputLocalPlayerSubsystem` (`GameplayStatics.GetPlayerController` 0)) "/Game/FPS_GAME/Data/IMC_FPS.IMC_FPS" 0 (struct))
  (`self.Spawn Inventory`)
  ; Create UI
  (bind _returnvalue (`|CreateWidget` "/Game/FPS_GAME/Core/WBP_PlayerUI.WBP_PlayerUI_C" (`GameplayStatics.GetPlayerController` 0)))
  (`UserWidget.AddToViewport` _returnvalue 0)
  (`self.Holster toggle`))

(event `EnhancedInput|/Game/FPS_GAME/Data/IA_Shoot`
  (params (ActionValue :type Boolean) (ElapsedSeconds :type "Float (double-precision)") (TriggeredSeconds :type "Float (double-precision)") (InputAction :type "InputAction Object Reference" :default "/Game/FPS_GAME/Data/IA_Shoot.IA_Shoot"))
  (bind _returnvalue (`SceneComponent.K2_GetComponentLocation` (`self.Camera`)))
  ; Shoot
  (:`Triggered`
    (`/Engine/EditorBlueprintResources/StandardMacros.DoOnce` false :!label _label
      (:`Completed`
        (set `self.bHoldingShoot` true)
        (if (and (and (and (> (`self.CurrentAmmunition`) 0) (and (`self.bHoldingShoot`) (not (`self.bRunning`)) (not (`self.bCloseToWall`)))) (not (`self.bReloading`))) (`self.bEquipped`)) :!label _label_2
          (message `/Game/FPS_GAME/Core/BPI_Weapon.Shoot` (`|GetArrayItem` (`self.EquippedWeapons`) (`self.EquippedWeaponIndex`)))
          (`|PlayMontage` (`self.Character Arms`) "/Game/FPS_GAME/Art/AssaultRifle/Animations/AM_FP_AssaultRifle_Fire_Montage.AM_FP_AssaultRifle_Fire_Montage"
            (:`then`
              (`|ExecutionSequence`
                (:`then_0`
                  (bind (_outhit _returnvalue_2) (`KismetSystemLibrary.LineTraceSingle` _returnvalue (+ (* (`SceneComponent.GetForwardVector` (`self.Camera`)) (`self.TraceDistance`)) _returnvalue) "TraceTypeQuery1" false (`self.EquippedWeapons`)))
                  (if _returnvalue_2
                    (bind (_bblockinghit _binitialoverlap _time _distance _location _impactpoint _normal _impactnormal _physmat _hitactor _hitcomponent) (`GameplayStatics.BreakHitResult` _outhit))
                    (`NiagaraFunctionLibrary.SpawnSystemAtLocation` "/Game/FPS_GAME/Art/VFX/NS_MuzzleFlash.NS_MuzzleFlash" _impactpoint (struct) (0.3 0.3 0.3))
                    (bind _returnvalue_3 (`|SpawnActorFromClass` "/Game/FPS_GAME/Core/FS_MasterField_Bullet.FS_MasterField_Bullet_C" (`KismetMathLibrary.MakeTransform` _impactpoint) "AlwaysSpawn" "MultiplyWithRoot" null null))
                    (set `self.Field` _returnvalue_3)
                    (`/Engine/EditorResources/FieldNodes/FS_MasterField.CE_Trigger` (`self.Field`))
                    (`GameplayStatics.ApplyDamage` _hitactor 50.0 null self)
                    (if (`SceneComponent.IsSimulatingPhysics` _hitcomponent "None")
                      (`PrimitiveComponent.AddImpulseAtLocation` _hitcomponent (* (`SceneComponent.GetForwardVector` (`self.Camera`)) (`self.InpulseDistance`)) _impactpoint "None")
                      (`PrimitiveComponent.IgnoreActorWhenMoving` (`self.CapsuleComponent`) null true :!label _label_3)
                      (bind _returnvalue_4 (`NiagaraFunctionLibrary.SpawnSystemAttached` "/Game/FPS_GAME/Art/VFX/NS_MuzzleFlash.NS_MuzzleFlash" (`Actor.RootComponent` (`|GetArrayItem` (`self.EquippedWeapons`) (`self.EquippedWeaponIndex`))) "None" (0.0 100.0 0.0) (struct) "SnapToTargetIncludingScale"))
                      (`SceneComponent.SetWorldScale3D` _returnvalue_4 (0.3 0.3 0.3))
                      (set `self.CurrentAmmunition` (- (`self.CurrentAmmunition`) 1))
                      (`KismetSystemLibrary.Delay` (`self.FireDelay`))
                      (goto _label_2))))
                (:`then_1`
                  (goto _label_3)))))))))
  (:`Completed`
    (set `self.bHoldingShoot` false)
    (goto _label :!via `Reset`)))

(event `EnhancedInput|/Game/FPS_GAME/Data/IA_Movement`
  (params (ActionValue :type "Vector2D Structure") (ElapsedSeconds :type "Float (double-precision)") (TriggeredSeconds :type "Float (double-precision)") (InputAction :type "InputAction Object Reference" :default "/Game/FPS_GAME/Data/IA_Movement.IA_Movement"))
  (bind (_x _y) (`KismetMathLibrary.BreakVector2D` (`self.MoveInput`)))
  ;[0.15 0.1384 0.03434 0.502] Character Movement
  (:`Triggered`
    (set `self.MoveInput` ActionValue :!label _label_4)
    (`self.AddMovementInput` (* _y (`self.GetActorForwardVector`)))
    (`self.AddMovementInput` (* _x (`self.GetActorRightVector`))))
  (:`Completed`
    (goto _label_4)))

(event `EnhancedInput|/Game/FPS_GAME/Data/IA_Camera`
  (params (ActionValue :type "Vector2D Structure") (ElapsedSeconds :type "Float (double-precision)") (TriggeredSeconds :type "Float (double-precision)") (InputAction :type "InputAction Object Reference" :default "/Game/FPS_GAME/Data/IA_Camera.IA_Camera"))
  (bind (_x _y) (`KismetMathLibrary.BreakVector2D` (`self.MouseInput`)))
  ;[0.15 0.1384 0.03434 0.502] Camera Movement
  (:`Triggered`
    (set `self.bUsingGamepad` false :!label _label_5)
    (set `self.MouseInput` ActionValue)
    (`self.AddControllerPitchInput` (* _y -1.0))
    (`self.AddControllerYawInput` _x))
  (:`Completed`
    (goto _label_5)))

(event `EnhancedInput|/Game/FPS_GAME/Data/IA_Gamepad`
  (params (ActionValue :type "Vector2D Structure") (ElapsedSeconds :type "Float (double-precision)") (TriggeredSeconds :type "Float (double-precision)") (InputAction :type "InputAction Object Reference" :default "/Game/FPS_GAME/Data/IA_Gamepad.IA_Gamepad"))
  (bind (_x _y) (`KismetMathLibrary.BreakVector2D` ActionValue))
  (bind _returnvalue (`KismetMathLibrary.SelectFloat` (`self.FrictionMultiplier`) 1.0 (`KismetSystemLibrary.IsValid` (`self.AssistTarget`))))
  ;[0.04061 0.15 0.0602 0.5] Gamepad Camera Movement
  (:`Triggered`
    (set `self.bUsingGamepad` true)
    (`self.AddControllerYawInput` (* _returnvalue _x))
    (`self.AddControllerPitchInput` (* (* _y _returnvalue) -1.0))))

(event `EnhancedInput|/Game/FPS_GAME/Data/IA_Reload`
  (params (ActionValue :type Boolean) (ElapsedSeconds :type "Float (double-precision)") (TriggeredSeconds :type "Float (double-precision)") (InputAction :type "InputAction Object Reference" :default "/Game/FPS_GAME/Data/IA_Reload.IA_Reload"))
  ; Reload
  (:`Triggered`
    (`/Engine/EditorBlueprintResources/StandardMacros.DoOnce` false :!label _label_6
      (:`Completed`
        (if (and (not (`self.bReloading`)) (`self.bEquipped`))
          (set `self.bReloading` true)
          (`|PlayMontage` (`self.Character Arms`) "/Game/FPS_GAME/Art/AssaultRifle/Animations/AM_FP_AssaultRifle_Reload.AM_FP_AssaultRifle_Reload"
            (:`then`
              (message `/Game/FPS_GAME/Core/BPI_Weapon.Reload` (`|GetArrayItem` (`self.EquippedWeapons`) (`self.EquippedWeaponIndex`)))
              (`KismetSystemLibrary.Delay` 1.85)
              (set `self.CurrentAmmunition` (`self.TotalAmmunition`)))
            (:`OnBlendOut`
              (set `self.bReloading` false)))))))
  (:`Completed`
    (goto _label_6 :!via `Reset`)))

(event `EnhancedInput|/Game/FPS_GAME/Data/IA_Run`
  (params (ActionValue :type Boolean) (ElapsedSeconds :type "Float (double-precision)") (TriggeredSeconds :type "Float (double-precision)") (InputAction :type "InputAction Object Reference" :default "/Game/FPS_GAME/Data/IA_Run.IA_Run"))
  ;[0.15 0.1384 0.03434 0.502] Running and FOV
  (:`Triggered`
    (if (`NavMovementInterface.IsFalling` (`self.CharacterMovement`))
      _
      (elif (not (`self.bCrouching`))
        (set `self.bRunning` true)
        (set `CharacterMovementComponent.MaxWalkSpeed` (`self.RunningSpeed`) (`self.CharacterMovement`))
        (bind (_direction _fov) (`Timeline|Timeline` :!label _label_7)
          (:`Update`
            (set `PlayerCameraManager.DefaultFOV` _fov (`GameplayStatics.GetPlayerCameraManager` 0)))))))
  (:`Completed`
    (`self.Stop Running`)))

(event `Stop Running`
  ;[0.15 0.1384 0.03434 0.502] Running and FOV
  (set `self.bRunning` false)
  (set `CharacterMovementComponent.MaxWalkSpeed` 600.0 (`self.CharacterMovement`))
  (goto _label_7 :!via `Reverse`))

(event `Holster toggle`
  ; Holster
  (set `self.bEquipped` (not (`self.bEquipped`)) :!label _label_8)
  (`|PlayMontage` (`self.Character Arms`) (select `bool` (`self.bEquipped`) :`false` "/Game/FPS_GAME/Art/AssaultRifle/Animations/AM_FP_AssaultRifle_Holster.AM_FP_AssaultRifle_Holster" :`true` "/Game/FPS_GAME/Art/AssaultRifle/Animations/AM_FP_AssaultRifle_Equip.AM_FP_AssaultRifle_Equip" :!type "AnimMontage Object Reference")))

(event `EnhancedInput|/Game/FPS_GAME/Data/IA_Jumping`
  (params (ActionValue :type Boolean) (ElapsedSeconds :type "Float (double-precision)") (TriggeredSeconds :type "Float (double-precision)") (InputAction :type "InputAction Object Reference" :default "/Game/FPS_GAME/Data/IA_Jumping.IA_Jumping"))
  ;[0.15 0.1384 0.03434 0.502] Jumping
  (:`Triggered`
    (`self.Jump`)
    (`self.Stop Running`))
  (:`Completed`
    (`self.StopJumping`)))

(event `End Slide`
  ; Comment
  (if (`self.bIsSliding`)
    (set `self.bIsSliding` false)
    (set `CharacterMovementComponent.GroundFriction` 8.0 (`self.CharacterMovement`))
    (set `CharacterMovementComponent.BrakingDecelerationWalking` 2048.0 (`self.CharacterMovement`))))

(event `EnhancedInput|/Game/FPS_GAME/Data/IA_Holster`
  (params (ActionValue :type Boolean) (ElapsedSeconds :type "Float (double-precision)") (TriggeredSeconds :type "Float (double-precision)") (InputAction :type "InputAction Object Reference" :default "/Game/FPS_GAME/Data/IA_Holster.IA_Holster"))
  ; Holster
  (:`Triggered`
    (`/Engine/EditorBlueprintResources/StandardMacros.DoOnce` false :!label _label_9
      (:`Completed`
        (goto _label_8))))
  (:`Completed`
    (goto _label_9 :!via `Reset`)))

(event `Start Slide`
  ; Comment
  (set `self.bIsSliding` true)
  (set `CharacterMovementComponent.GroundFriction` 0.0 (`self.CharacterMovement`))
  (set `CharacterMovementComponent.BrakingDecelerationWalking` 300.0 (`self.CharacterMovement`))
  (`self.LaunchCharacter` (* (`KismetMathLibrary.Normal` (`self.GetVelocity`)) (`self.SlideSpeed`)) true)
  (`KismetSystemLibrary.Delay` (`self.SlideDuration`))
  (`self.End Slide`))

(event `EnhancedInput|/Game/FPS_GAME/Data/IA_Crouch`
  (params (ActionValue :type Boolean) (ElapsedSeconds :type "Float (double-precision)") (TriggeredSeconds :type "Float (double-precision)") (InputAction :type "InputAction Object Reference" :default "/Game/FPS_GAME/Data/IA_Crouch.IA_Crouch"))
  ;[0.15 0.1384 0.03434 0.502] Crouching
  (:`Triggered`
    (`/Engine/EditorBlueprintResources/StandardMacros.DoOnce` false :!label _label_10
      (:`Completed`
        (if (`self.bHoldCrouch`)
          (`self.Custom Crouch`)
          (else
            (`/Engine/EditorBlueprintResources/StandardMacros.FlipFlop`
              (:`A`
                (`self.Custom Crouch`))
              (:`B`
                (`self.Custom Un Crouch`))))))))
  (:`Completed`
    (`|ExecutionSequence`
      (:`then_0`
        (if (`self.bHoldCrouch`)
          (`self.Custom Un Crouch`)))
      (:`then_1`
        (goto _label_10 :!via `Reset`)))))

(event `Custom Crouch`
  ;[0.15 0.1384 0.03434 0.502] Crouching
  (if (and (> (`KismetMathLibrary.VSizeXY` (`self.GetVelocity`)) 700.0) (`NavMovementComponent.IsMovingOnGround` (`self.CharacterMovement`)) (not (`self.bIsSliding`)))
    (`self.Start Slide`))
  (set `self.bCrouching` true)
  (`self.Stop Running`)
  (set `CharacterMovementComponent.MaxWalkSpeed` 400.0 (`self.CharacterMovement`))
  (bind (_direction _half_height) (`Timeline|Crouch Timeline` :!label _label_11)
    (:`Update`
      (`CapsuleComponent.SetCapsuleHalfHeight` (`self.CapsuleComponent`) _half_height true))))

(event `Custom Un Crouch`
  ;[0.15 0.1384 0.03434 0.502] Crouching
  (`self.End Slide`)
  (set `self.bCrouching` false)
  (set `CharacterMovementComponent.MaxWalkSpeed` 600.0 (`self.CharacterMovement`))
  (goto _label_11 :!via `Reverse`))

(event `self.ReceiveTick`
  (params (DeltaSeconds :type "Float (single-precision)"))
  (bind _returnvalue (`GameplayStatics.GetPlayerCameraManager` 0))
  (bind _camera (`self.Camera`))
  ; Camera Rotation Fix
  (`SceneComponent.K2_SetRelativeRotation` (`self.Pivot`) (`KismetMathLibrary.MakeRotator` 0.0 (.pitch (`self.GetControlRotation`))) false false)
  ; Wall Sway
  (bind (_outhit _returnvalue_2) (`KismetSystemLibrary.LineTraceSingle` (`SceneComponent.K2_GetComponentLocation` (`self.Camera`)) (+ (`SceneComponent.K2_GetComponentLocation` _camera) (* (`SceneComponent.GetForwardVector` _camera) (100.0 100.0 100.0))) "TraceTypeQuery1"))
  (set `self.bCloseToWall` _returnvalue_2)
  ;[0.04061 0.15 0.0602 0.5] AimAsist Gamepad
  (`|ExecutionSequence`
    (:`then_0`
      (if (`self.bUsingGamepad`)
        (bind (_outhit_2 _returnvalue_3) (`KismetSystemLibrary.SphereTraceSingle` :`Start` (`PlayerCameraManager.GetCameraLocation` _returnvalue) :`End` (+ (`PlayerCameraManager.GetCameraLocation` _returnvalue) (* (`KismetMathLibrary.GetForwardVector` (`PlayerCameraManager.GetCameraRotation` _returnvalue)) (`self.AssistRange`))) :`Radius` (`self.AssistRadius`) :`TraceChannel` "TraceTypeQuery1" :`DrawDebugType` "ForOneFrame"))
        (if _returnvalue_3
          (bind (_bblockinghit _binitialoverlap _time _distance _location _impactpoint _normal _impactnormal _physmat _hitactor) (`GameplayStatics.BreakHitResult` _outhit_2))
          (if (`self.ActorHasTag` _hitactor "Enemy")
            (set `self.AssistTarget` _hitactor)
            (else
              (set `self.AssistTarget` null)))
          (else
            (set `self.AssistTarget` null)))
        (else
          (set `self.AssistTarget` null))))
    (:`then_1`
      (`self.AssistTarget`
        (:`then`
          (`Controller.SetControlRotation` (`GameplayStatics.GetPlayerController` 0) (`KismetMathLibrary.RInterpTo` (`self.GetControlRotation`) (`KismetMathLibrary.FindLookAtRotation` (`PlayerCameraManager.GetCameraLocation` (`GameplayStatics.GetPlayerCameraManager` 0)) (+ (`self.K2_GetActorLocation` (`self.AssistTarget`)) (`KismetMathLibrary.MakeVector` 0.0 0.0 (`self.AimHeightOffset`)))) (`GameplayStatics.GetWorldDeltaSeconds`) (`self.MagnetSpeed`))))
        (:`else`)))))

(event `EnhancedInput|/Game/FPS_GAME/Data/IA_Aim`
  (params (ActionValue :type Boolean) (ElapsedSeconds :type "Float (double-precision)") (TriggeredSeconds :type "Float (double-precision)") (InputAction :type "InputAction Object Reference" :default "/Game/FPS_GAME/Data/IA_Aim.IA_Aim"))
  ; Aiming
  (:`Triggered`
    (set `self.bAiming` true))
  (:`Completed`
    (set `self.bAiming` false)))

(fn `Spawn Inventory`
  ; Equipped Weapons
  (for _array_element (`self.Inventory`)
    (bind _returnvalue (`|SpawnActorFromClass` _array_element (`KismetMathLibrary.MakeTransform` (0.0 0.0 0.0)) "Undefined" "MultiplyWithRoot" null null))
    (`KismetArrayLibrary.Array_Add` (`self.EquippedWeapons`) _returnvalue)
    (`self.K2_AttachToComponent` _returnvalue (`self.Character Arms`) "ik_hand_gun" "KeepRelative" "KeepRelative" "KeepRelative" true)
    (`self.SetActorHiddenInGame` _returnvalue true))
  (`self.SetActorHiddenInGame` (`|GetArrayItem` (`self.EquippedWeapons`) (`self.EquippedWeaponIndex`)) false))

(fn `UserConstructionScript`)