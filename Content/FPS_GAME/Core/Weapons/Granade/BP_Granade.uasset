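; BP_Granade is a grenade actor that explodes on hit and pushes nearby AI characters.
; On hit it spawns a Niagara explosion, plays a sound, then destroys itself.
; A sphere overlap at its location finds BP_AI pawns and calls RadialImpulse on each with the impact location.
; A StartSpin event enables a steady pitch and yaw spin in Tick.
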(event `self.ReceiveHit`
  (params (MyComp :type "PrimitiveComponent Object Reference") (Other :type "Actor Object Reference") (OtherComp :type "PrimitiveComponent Object Reference") (bSelfMoved :type Boolean) (HitLocation :type "Vector Structure") (HitNormal :type "Vector Structure") (NormalImpulse :type "Vector Structure") (Hit :type "HitResult Structure (by ref)"))
  (bind (_bblockinghit _binitialoverlap _time _distance _location) (`GameplayStatics.BreakHitResult` Hit))
  (bind _location_2 (.location (`self.GetTransform`)))
  (`|ExecutionSequence`
    (:`then_0`
      (`NiagaraFunctionLibrary.SpawnSystemAtLocation` "/Game/FPS_GAME/Art/VFX/Explotion/NS_Explosion.NS_Explosion" _location_2)
      (`GameplayStatics.PlaySoundAtLocation` null _location (struct) 1.0 1.0 0.0 null null null null)
      (bind _outactors (`KismetSystemLibrary.SphereOverlapActors` _location_2 0.0 (`|MakeArray` "ObjectTypeQuery3" :!type "EObjectTypeQuery Enum") "/Game/FPS_GAME/Enemy_AI/BP_AI.BP_AI_C"))
      (for _array_element _outactors
        (bind _asbp_ai (cast `/Game/FPS_GAME/Enemy_AI/BP_AI` _array_element))
        (`/Game/FPS_GAME/Enemy_AI/BP_AI.RadialImpulse` _asbp_ai _location)))
    (:`then_1`
      (`self.K2_DestroyActor`))))

(event `StartSpin`
  (set `self.bStartSpin` true))

(event `self.ReceiveTick`
  (params (DeltaSeconds :type "Float (single-precision)"))
  (bind _returnvalue (* DeltaSeconds 360.0))
  (if (`self.bStartSpin`)
    (`self.K2_AddActorLocalRotation` (`KismetMathLibrary.MakeRotator` 0.0 _returnvalue _returnvalue))))

(fn `UserConstructionScript`)