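; BP_Weapon is an assault rifle weapon for an FPS, providing the animation and shell ejection side of shooting and reloading.
; Shoot plays the fire montage on the rifle mesh and spawns a BP_Casing at its ejection socket, with ignore-when-moving against the player explicitly off.
; Reload only plays the reload montage.
; The file contains no projectile, damage or ammo logic.
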(event `/Game/FPS_GAME/Core/BPI_Weapon.Shoot`
  ; Shoot
  (`|PlayMontage` (`self.SK_AssaultRifle`) "/Game/FPS_GAME/Art/AssaultRifle/Animations/AM_FP_WEP_AssaultRifle_Fire_Montage.AM_FP_WEP_AssaultRifle_Fire_Montage"
    (:`then`
      (bind _returnvalue (`|SpawnActorFromClass` "/Game/FPS_GAME/Core/BP_Casing.BP_Casing_C" (`SceneComponent.GetSocketTransform` (`self.SK_AssaultRifle`) "SOCKET_Ejection" "RTS_World") "AlwaysSpawn" "MultiplyWithRoot" null null))
      (`PrimitiveComponent.IgnoreActorWhenMoving` (`/Game/FPS_GAME/Core/BP_Casing.CasingMesh` _returnvalue) (`GameplayStatics.GetPlayerCharacter` 0) false))))

(event `/Game/FPS_GAME/Core/BPI_Weapon.Reload`
  (`|PlayMontage` (`self.SK_AssaultRifle`) "/Game/FPS_GAME/Art/AssaultRifle/Animations/AM_FP_WEP_AssaultRifle_Reload.AM_FP_WEP_AssaultRifle_Reload"))

(fn `UserConstructionScript`)